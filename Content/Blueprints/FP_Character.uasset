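; FP_Character is a player character Blueprint, named as first-person, that handles basic walking, sprinting and look controls.
; Forward and right axis inputs move the character along directions built from control rotation yaw only, so camera pitch does not affect movement.
; The Sprint action switches CharacterMovement's max walk speed between a faster and a normal value on press and release.
; Look axes feed controller pitch and yaw directly, and the construction script is empty.
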(event `InputAxis|MoveForward`
  (params (AxisValue :type "Float (single-precision)"))
  (bind (_returnvalue_roll _returnvalue_pitch _returnvalue_yaw) (`KismetMathLibrary.BreakRotator` (`self.GetControlRotation`)))
  ;[1 1 1] Movement
  (`self.AddMovementInput` (`KismetMathLibrary.GetForwardVector` (`KismetMathLibrary.MakeRotator` 0.0 0.0 _returnvalue_yaw)) AxisValue))

(event `InputAxis|MoveRight`
  (params (AxisValue :type "Float (single-precision)"))
  (bind (_returnvalue_roll _returnvalue_pitch _returnvalue_yaw) (`KismetMathLibrary.BreakRotator` (`self.GetControlRotation`)))
  ;[1 1 1] Movement
  (`self.AddMovementInput` (`KismetMathLibrary.GetRightVector` (`KismetMathLibrary.MakeRotator` 0.0 0.0 _returnvalue_yaw)) AxisValue))

(event `InputAction|Sprint`
  (params (Key :type "Key Structure"))
  (bind _charactermovement (`self.CharacterMovement`))
  ;[1 1 1] Movement
  (:`Pressed`
    (set `CharacterMovementComponent.MaxWalkSpeed` 500.0 _charactermovement))
  (:`Released`
    (set `CharacterMovementComponent.MaxWalkSpeed` 300.0 _charactermovement)))

(event `InputAxis|LookUp`
  (params (AxisValue :type "Float (single-precision)"))
  ;[1 1 1] Camera
  (`self.AddControllerPitchInput` AxisValue))

(event `InputAxis|LookRight`
  (params (AxisValue :type "Float (single-precision)"))
  ;[1 1 1] Camera
  (`self.AddControllerYawInput` AxisValue))

(fn `UserConstructionScript`)