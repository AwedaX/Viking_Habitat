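; BP_Visual_Visual_Cmds is a utility Blueprint that applies level-of-detail and ray tracing overrides through console commands.
; Change_LOD forces the LOD stored in LODs via r.ForceLOD, and Change_RT_Quality maps the RTQ enum to ForceAllRayTracingEffects for off, default or full ray tracing.
; Both events print the new setting, and a Stats event prints the two variables' current values.
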(event `Stats`
  (`KismetSystemLibrary.PrintString` (`KismetStringLibrary.Concat_StrStr` "LODs " (`KismetStringLibrary.Conv_IntToString` (`self.LODs`)) " \n" "RT Quality - " (`|GetEnumeratorNameAsString` (`self.RTQ`))) true true (struct :`G` 0.66 :`B` 1.0 :`A` 1.0) 3.0))

(event `Change_LOD`
  (bind _returnvalue (`KismetStringLibrary.Conv_IntToString` (`self.LODs`)))
  (`KismetSystemLibrary.ExecuteConsoleCommand` (`KismetStringLibrary.Concat_StrStr` "r.Forcelod " _returnvalue) null)
  (`KismetSystemLibrary.PrintString` (`KismetStringLibrary.Concat_StrStr` "LODs Changed to LODs " _returnvalue) true true (struct :`G` 0.66 :`B` 1.0 :`A` 1.0) 3.0))

(event `Change_RT_Quality`
  (bind _rtq (`self.RTQ`))
  (switch `/Game/Blueprints/Visual_Visual_Cmds/E_RTQ` _rtq
    (:`NewEnumerator0`
      (`KismetSystemLibrary.ExecuteConsoleCommand` "r.RayTracing.ForceAllRayTracingEffects 0" null))
    (:`NewEnumerator1`
      (`KismetSystemLibrary.ExecuteConsoleCommand` "r.RayTracing.ForceAllRayTracingEffects -1" null))
    (:`NewEnumerator2`
      (`KismetSystemLibrary.ExecuteConsoleCommand` "r.RayTracing.ForceAllRayTracingEffects 1" null)))
  (`KismetSystemLibrary.PrintString` (`KismetStringLibrary.Concat_StrStr` "RT Quality Changed to - " (`|GetEnumeratorNameAsString` _rtq)) true true (struct :`G` 0.66 :`B` 1.0 :`A` 1.0) 3.0))

(fn `UserConstructionScript`)