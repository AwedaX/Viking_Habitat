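; Blueprint of visual quality presets that switches LOD and ray tracing settings through console commands.
; Separate events force mesh and foliage LOD to cinematic detail, LOD 2, or the default gameplay behavior.
; Ray tracing events force all effects on, off, or back to default, and store a Full, Basic or No Raytracing label in RaytracingCurrentState.
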(event `Cinematic LOD`
  (`KismetSystemLibrary.ExecuteConsoleCommand` "r.Forcelod 0" null))

(event `Cinematic Foliage LOD`
  (`KismetSystemLibrary.ExecuteConsoleCommand` "foliage.ForceLOD 0" null))

(event `Full Raytracing`
  (`KismetSystemLibrary.ExecuteConsoleCommand` "r.RayTracing.ForceAllRayTracingEffects 1" null)
  (set `self.Raytracing current state` "Full Raytracing"))

(event `Gameplay LOD`
  (`KismetSystemLibrary.ExecuteConsoleCommand` "r.Forcelod -1" null))

(event `Gameplay  Foliage LOD`
  (`KismetSystemLibrary.ExecuteConsoleCommand` "foliage.ForceLOD -1" null))

(event `Basic Raytracing`
  (`KismetSystemLibrary.ExecuteConsoleCommand` "r.RayTracing.ForceAllRayTracingEffects -1" null)
  (set `self.Raytracing current state` "Basic Raytracing"))

(event `LOD 2`
  (`KismetSystemLibrary.ExecuteConsoleCommand` "r.Forcelod 2" null))

(event `Foliage LOD 2`
  (`KismetSystemLibrary.ExecuteConsoleCommand` "foliage.ForceLOD 2" null))

(event `No Raytracing`
  (`KismetSystemLibrary.ExecuteConsoleCommand` "r.RayTracing.ForceAllRayTracingEffects 0" null)
  (set `self.Raytracing current state` "No Raytracing"))

(fn `UserConstructionScript`)